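; BP_LlamaTest is a test Blueprint that exercises a Llama language-model component.
; On BeginPlay it prints a greeting, starts loading the model and binds handlers for model-loaded, token-generated and response-generated events.
; Once the model loads it inserts a templated one-sentence greeting prompt, then prints each token and response as it arrives.
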(event Custom|OnModelLoaded_Event
  (params (ModelName :type String))
  (Class|LlamaComponent|InsertTemplatedPrompt (Variables|Default|GetLlama) "Hello! Say hi in one sentence." "User" false true))

(event Custom|OnTokenGenerated_Event
  (params (Token :type String))
  (Development|PrintString Token))

(event Custom|OnResponseGenerated_Event
  (params (Response :type String))
  (Development|PrintString Response))

(event EventBeginPlay
  (bind _llama (Variables|Default|GetLlama))
  (Development|PrintString "Hello")
  (Class|LlamaComponent|LoadModel _llama true)
  (EventDispatchers|AssignOnModelLoaded _llama (delegate Custom|OnModelLoaded_Event))
  (EventDispatchers|AssignOnTokenGenerated _llama (delegate Custom|OnTokenGenerated_Event))
  (EventDispatchers|AssignOnResponseGenerated _llama (delegate Custom|OnResponseGenerated_Event)))

(event Collision|EventActorBeginOverlap
  (params (OtherActor :type Actor%20Object%20Reference)))

(event EventTick
  (params (DeltaSeconds :type Float%20%28single-precision%29)))

(fn ConstructionScript)