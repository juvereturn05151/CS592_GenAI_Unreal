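; Actor that runs a chat screen for a local Llama language model, creating WBP_Chat and loading the model on BeginPlay.
; Once loaded, Send replaces the history with the user's message and submits it as a templated prompt.
; Streamed tokens accumulate in a buffer, with a short timer meant to throttle UI refreshes, though its pending flag is never reset.
; Completed responses append to the history and scroll the chat down.
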(event Custom|UpdateChatUI_Timer
  (Variables|/Script/UMG.TextBlock|SetText (Variables|/Game/Blueprints/WBP_Chat.WBP_Chat_C|GetChatText (Variables|Default|GetChatWidget)) (Utilities|Text|ToText(String) (Utilities|String|Append (Variables|Default|GetChatHistory) (Variables|Default|GetCurrentAssistant)))))

(event Custom|OnClickSent
  (CallFunction|WhenClickSent))

(event Custom|OnTokenGeneratedEvent
  (params (Token :type String))
  (CallFunction|WhenTokenGenerated Token))

(event Custom|OnResponseGenerated
  (params (Response :type String))
  (CallFunction|WhenResponseGenerated Response))

(event Custom|FinishLoading
  (params (ModelName :type String))
  (bind _llama (Variables|Default|GetLlama))
  (EventDispatchers|BindEventtoOnClicked (Variables|/Game/Blueprints/WBP_Chat.WBP_Chat_C|GetSendButton (Variables|Default|GetChatWidget)) (delegate Custom|OnClickSent))
  (EventDispatchers|BindEventtoOnTokenGenerated _llama (delegate Custom|OnTokenGeneratedEvent))
  (EventDispatchers|BindEventtoOnResponseGenerated _llama (delegate Custom|OnResponseGenerated)))

(event EventBeginPlay
  (bind _llama (Variables|Default|GetLlama))
  (bind _returnvalue (UserInterface|CreateWidget "/Game/Blueprints/WBP_Chat.WBP_Chat_C"))
  (bind _output_get (Variables|Default|SetChatWidget _returnvalue))
  (UserInterface|Viewport|AddtoViewport _output_get 0)
  (Class|LlamaComponent|LoadModel _llama true)
  (EventDispatchers|BindEventtoOnModelLoaded _llama (delegate Custom|FinishLoading)))

(event Collision|EventActorBeginOverlap
  (params (OtherActor :type Actor%20Object%20Reference)))

(event EventTick
  (params (DeltaSeconds :type Float%20%28single-precision%29)))

(fn ConstructionScript)

(fn WhenTokenGenerated
  (params (Tokens :type String))
  (Variables|Default|SetCurrentAssistant (Utilities|String|Append (Variables|Default|GetCurrentAssistant) Tokens))
  (if (not (Variables|Default|GetPendingUIUpdate))
    (Variables|Default|SetPendingUIUpdate true)
    (Utilities|Time|SetTimerbyEvent (EventDispatchers|CreateEvent :!event Custom|UpdateChatUI_Timer) 0.05)))

(fn WhenResponseGenerated
  (params (Response :type String))
  (bind _output_get (Variables|Default|SetChatHistory (Utilities|String|Append (Variables|Default|GetChatHistory) (Variables|Default|GetCurrentAssistant) "\\n")))
  (Variables|/Script/UMG.TextBlock|SetText (Variables|/Game/Blueprints/WBP_Chat.WBP_Chat_C|GetChatText (Variables|Default|GetChatWidget)) (Utilities|Text|ToText(String) _output_get))
  (Variables|Default|SetCurrentAssistant "")
  (Class|ScrollBox|ScrolltoEnd (Variables|/Game/Blueprints/WBP_Chat.WBP_Chat_C|GetChatScroll (Variables|Default|GetChatWidget))))

(fn WhenClickSent
  (bind _chatwidget (Variables|Default|GetChatWidget))
  (bind _inputbox (Variables|/Game/Blueprints/WBP_Chat.WBP_Chat_C|GetInputBox _chatwidget))
  (if (not (Utilities|Array|IsEmpty (Utilities|String|ToString(Text) (Variables|/Script/UMG.EditableTextBox|GetText _inputbox))))
    (bind _output_get (Variables|Default|SetChatHistory (Utilities|String|Append "User: " (Utilities|String|ToString(Text) (Variables|/Script/UMG.EditableTextBox|GetText _inputbox)))))
    (bind _output_get_2 (Variables|/Script/UMG.TextBlock|SetText (Variables|/Game/Blueprints/WBP_Chat.WBP_Chat_C|GetChatText _chatwidget) (Utilities|Text|ToText(String) _output_get)))
    (Development|PrintText _output_get_2)
    (Variables|/Script/UMG.EditableTextBox|SetText _inputbox "")
    (Class|LlamaComponent|InsertTemplatedPrompt (Variables|Default|GetLlama) (Utilities|String|ToString(Text) _output_get_2) "User" false true)
    (Variables|Default|SetCurrentAssistant "")
    (Development|PrintString "Insert Success")))